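; Player controller that runs a paddle-and-ball style level with HUD, movement input and win/lose screens.
; On start it shows the HUD and listens for the cube generator's all-cubes-died event as a win.
; On possess it binds the pawn's game-over event as a loss; both outcomes share one path that shows the win screen in UI-only mode.
; Input slides the pawn sideways with sweep, spawns balls, or exits to the menu.
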(event Custom|GameFinished
  (Variables|Default|SetbIsWinner true)
  (Widget|SetVisibility (Variables|Default|GetHUD) "Collapsed")
  (bind _returnvalue (UserInterface|CreateWidget "/Game/MyGame/UI/WBP_WinScreen.WBP_WinScreen_C" self))
  (Default|UpdateWinner _returnvalue (Variables|Default|GetbIsWinner))
  (UserInterface|Viewport|AddtoViewport _returnvalue 0)
  (Input|SetInputModeUIOnly self 0 "LockOnCapture")
  (Variables|Default|SetbShowMouseCursor true))

(event Custom|PlayerDie
  (Variables|Default|SetbIsWinner false)
  (Widget|SetVisibility (Variables|Default|GetHUD) "Collapsed")
  (bind _returnvalue (UserInterface|CreateWidget "/Game/MyGame/UI/WBP_WinScreen.WBP_WinScreen_C" self))
  (Default|UpdateWinner _returnvalue (Variables|Default|GetbIsWinner))
  (UserInterface|Viewport|AddtoViewport _returnvalue 0)
  (Input|SetInputModeUIOnly self 0 "LockOnCapture")
  (Variables|Default|SetbShowMouseCursor true))

(event EventBeginPlay
  (Utilities|FlowControl|Sequence
    (:then_0
      (Input|SetInputModeGameOnly self)
      (bind _returnvalue (UserInterface|CreateWidget "/Game/MyGame/UI/WBP_HUD.WBP_HUD_C" self))
      (UserInterface|Viewport|AddtoViewport _returnvalue 0)
      (Variables|Default|SetHUD _returnvalue))
    (:then_1
      (bind _returnvalue_2 (Actor|GetActorOfClass "/Game/MyGame/Blueprints/BP_CubesGenerator.BP_CubesGenerator_C"))
      (EventDispatchers|BindEventtoAllCubesDied _returnvalue_2 (delegate Custom|GameFinished)))))

(event EventPossess
  (params (PossessedPawn :type Pawn%20Object%20Reference))
  (bind _asbp_my_pawn (Utilities|Casting|CastToBP_MyPawn PossessedPawn))
  (bind _output_get (Variables|Default|SetMyPawn _asbp_my_pawn))
  (EventDispatchers|BindEventtoGameOver _output_get (delegate Custom|PlayerDie)))

(event Input|ActionEvents|InputActionSpawnBall
  (params (Key :type Key%20Structure :default "None"))
  (:Pressed
    (Default|SpawnBall (Variables|Default|GetMyPawn))))

(event Input|ActionEvents|InputActionExit
  (params (Key :type Key%20Structure :default "None"))
  (:Pressed
    (Game|OpenLevel(byObjectReference) "/Game/MyGame/Levels/MENU.MENU")))

(event Input|AxisEvents|InputAxisLeft_Right
  (params (AxisValue :type Float%20%28single-precision%29))
  (Transformation|AddActorWorldOffset (Variables|Default|GetMyPawn) (Math|Vector|MakeVector 0.0 (* AxisValue (Utilities|Time|GetWorldDeltaSeconds) (Variables|Default|GetSpeed)) 0.0) true))

(fn ConstructionScript)