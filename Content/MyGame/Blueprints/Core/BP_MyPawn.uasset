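; Player paddle pawn for a ball-and-bonus game, tracking lives and score and launching balls from an arrow.
; SpawnBall allows one tracked ball at a time; its destruction costs HP and either re-shows the SPACE prompt or signals game over.
; Overlapping bonuses add score and trigger a timed paddle widening, an extra life or a smaller, untracked extra ball.
; HP, score and game-over changes go out through Call events.
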(event OnComponentBeginOverlap(Cube)
  (params (OverlappedComponent :type Primitive%20Component%20Object%20Reference) (OtherActor :type Actor%20Object%20Reference) (OtherComp :type Primitive%20Component%20Object%20Reference) (OtherBodyIndex :type Integer) (bFromSweep :type Boolean) (SweepResult :type Hit%20Result%20Structure%20%28by%20ref%29))
  (bind _asbp_bonus (Utilities|Casting|CastToBP_Bonus OtherActor))
  (switch Utilities|FlowControl|Switch|SwitchonE_BonusType (Variables|/Game/MyGame/Blueprints/Bonuses/BP_Bonus.BP_Bonus_C|GetBonusType _asbp_bonus)
    (:NewEnumerator0
      (CallFunction|+SIZEEvent))
    (:NewEnumerator1
      (CallFunction|+HPEvent))
    (:NewEnumerator2
      (CallFunction|+BALLEvent)))
  (CallFunction|AddedScore 50)
  (Audio|PlaySoundatLocation "/Game/MyGame/Sounds/A_Bonus_Cue.A_Bonus_Cue" (Transformation|GetActorLocation) "0, 0, 0" 1.0 1.0 0.0 0 0 0)
  (Actor|DestroyActor _asbp_bonus))

(event Custom|SpawnBall
  (if (not (<= (Variables|Default|GetHP) 0))
    (Variables|Default|GetAliveBall
      (:then)
      (:else
        (bind _returnvalue (Game|SpawnActorfromClass "/Game/MyGame/Blueprints/BP_Ball.BP_Ball_C" (Math|Transform|MakeTransform (Transformation|GetWorldLocation (Variables|Default|GetArrow))) "Undefined" 0 0))
        (bind _output_get (Variables|Default|SetAliveBall _returnvalue))
        (Game|BindEventtoOnDestroyed _output_get (delegate Custom|BallisDead))
        (Rendering|SetVisibility (Variables|Default|GetSPACE) false false)))))

(event Custom|BallisDead
  (params (DestroyedActor :type Actor%20Object%20Reference))
  (bind _result (Math|Integer|DecrementInt (Variables|Default|GetHP))
    (:%20%20
      (Default|CallHPChanged _result)
      (if (<= _result 0)
        (Default|CallGameOver)
        (else
          (Rendering|SetVisibility (Variables|Default|GetSPACE) true false)
          (Audio|PlaySoundatLocation "/Game/MyGame/Sounds/A_Dead_Cue.A_Dead_Cue" (Transformation|GetActorLocation) "0, 0, 0" 1.0 1.0 0.0 0 0 0))))))

(event Custom|+SIZE_Event
  (bind _cube (Variables|Default|GetCube))
  (bind _relativescale3d (Variables|/Script/Engine.SceneComponent|GetRelativeScale3D _cube))
  (Transformation|SetRelativeScale3D _cube (Math|Vector|MakeVector (.x _relativescale3d) (* (.y _relativescale3d) 1.2) (.z _relativescale3d)))
  (CallFunction|-SIZEEvent))

(event Custom|+HP_Event
  (bind _result (Math|Integer|IncrementInt (Variables|Default|GetHP))
    (:%20%20
      (Default|CallHPChanged _result))))

(event Custom|+BALL_Event
  (Game|SpawnActorfromClass "/Game/MyGame/Blueprints/BP_Ball.BP_Ball_C" (Math|Transform|MakeTransform (Transformation|GetWorldLocation (Variables|Default|GetArrow)) "0, 0, 0" "0.500000,0.500000,0.500000") "Undefined" 0 0))

(event Custom|-SIZE_Event
  (Utilities|FlowControl|RetriggerableDelay 1e+01)
  (Transformation|SetRelativeScale3D (Variables|Default|GetCube) (Variables|Default|GetDefaultScale)))

(event EventBeginPlay
  (Variables|Default|SetDefaultScale (Variables|/Script/Engine.SceneComponent|GetRelativeScale3D (Variables|Default|GetCube))))

(fn ConstructionScript)

(fn AddedScore
  (params (Amount :type Integer))
  (bind _output_get (Variables|Default|SetAllScore (+ (Variables|Default|GetAllScore) (Math|Integer|Absolute(Integer) Amount))))
  (Default|CallScoreChanged _output_get))