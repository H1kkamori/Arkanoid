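; BP_Bonus is a bonus actor that gets one of three random types and moves along the X axis.
; The construction script picks BonusType at random and shows its enum name on a TextRender.
; Each tick offsets the Cylinder component with sweep, using only the X component of Direction scaled by Speed and delta time.
; The file contains no pickup or effect logic.
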(event EventTick
  (params (DeltaSeconds :type Float%20%28single-precision%29))
  (Transformation|AddWorldOffset (Variables|Default|GetCylinder) (Math|Vector|MakeVector (.x (* (Variables|Default|GetDirection) (* DeltaSeconds (Variables|Default|GetSpeed)))) 0.0 0.0) true false))

(fn ConstructionScript
  (Variables|Default|SetBonusType (Utilities|Select :Index (Math|Random|RandomIntegerinRange 0 2) :Option%200 "NewEnumerator0" :Option%201 "NewEnumerator1" :Option%202 "NewEnumerator2"))
  (Rendering|Components|TextRender|SetText (Variables|Default|GetTextRender) (Utilities|Text|ToText(String) (Utilities|String|EnumtoString (Variables|Default|GetBonusType)))))